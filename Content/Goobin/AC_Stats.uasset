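; AC_Stats is an actor component that tracks an owner's health and applies damage to it.
; AffectHealth subtracts a value, clamps Health between zero and MaxHealth, then fires OnDamaged and, at zero, OnDepleted.
; IsAlive reports whether Health remains and, when DestroyOnDeplete is set, destroys the owning actor on depletion, which happens before the damage events broadcast.
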(fn `AffectHealth`
  (params (Value :type "Float (double-precision)"))
  (returns (OutHealth :type "Float (double-precision)"))
  (bind _health (`self.Health`))
  (set `self.Health` (`KismetMathLibrary.FClamp` (- (`self.Health`) Value) 0.0 (`self.MaxHealth`)))
  (`self.IsAlive`)
  (`self.OnDamaged` _health (`local.Value`))
  (if (<= _health 0.0)
    (`self.OnDepleted`))
  (return (`self.Health`)))

(fn `IsAlive`
  (returns (IsAlive :type Boolean))
  (if (> (`self.Health`) 0.0)
    (return true)
    (elif (`self.DestroyOnDeplete`)
      (`Actor.K2_DestroyActor` (`self.GetOwner`))
      (return false)
      (else
        (return false)))))