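; Dialogue component for the War Chief Goobin, who asks the player whether they want to go to war.
; It overrides the parent Dialogue function, calling it first, then branches on the dialogue tree index and the chosen option of each AddDialogue line.
; Accepting opens the Arena level, while declining shows a dismissive reply; both paths clear dialogue progress and close the conversation.
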(fn `Dialogue`
  (`parent.Dialogue`)
  (switch `int` (`self.DialogueTreeIndex`)
    (:`0`
      (bind (_state _optionindex) (`self.AddDialogue` (`self.Character Name`) "Hi fellow! Want to war?" (`|MakeArray` "Yes! I love war!" "No, I want peace." :!type "Text")))
      (switch `/Game/Goobin/Dialogue/E_DialogueState` _state
        (:`NewEnumerator0`
          (switch `int` _optionindex
            (:`0`
              (`GameplayStatics.OpenLevel` "Arena")
              (`self.ClearDialogueProgress`)
              (`self.CloseConversation`))
            (:`1`
              (bind _state_2 (`self.AddDialogue` (`self.Character Name`) "Gah! This Goobin is no war-fighter. Come back when strong!" (`|MakeArray` "Continue" :!type "Text")))
              (switch `/Game/Goobin/Dialogue/E_DialogueState` _state_2
                (:`NewEnumerator0`
                  (`self.ClearDialogueProgress`)
                  (`self.CloseConversation`))))))))))