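; Test NPC dialogue component that scripts a goobin conversation about building a home in the village.
; It caches BP_Village on BeginPlay and overrides Dialogue, branching on the saved tree index and chosen options.
; Asking for a home checks Wood and Rock costs through the village, then creates a test building or refuses.
; Insulting the NPC switches to a tree where it refuses to talk.
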(event `self.ReceiveBeginPlay`
  (bind _returnvalue (`GameplayStatics.GetActorOfClass` "/Game/Goobin/Blueprints/BP_Village.BP_Village_C"))
  (set `self.Village` _returnvalue))

(fn `Dialogue`
  (bind _village (`self.Village`))
  (`parent.Dialogue`)
  (switch `int` (`self.DialogueTreeIndex`)
    (:`0`
      (bind (_state _optionindex) (`self.AddDialogue` (`self.Character Name`) "What want?" (`|MakeArray` "You're dumb" "I want make home" :!type "Text")))
      (switch `/Game/Goobin/Dialogue/E_DialogueState` _state
        (:`NewEnumerator0`
          (switch `int` _optionindex
            (:`0`
              (bind _state_2 (`self.AddDialogue` (`self.Character Name`) "You goobin suck! no TALK!" (`|MakeArray` "Continue" :!type "Text")))
              (switch `/Game/Goobin/Dialogue/E_DialogueState` _state_2
                (:`NewEnumerator0`
                  (`self.SetDialogueTreeIndex` 1)
                  (`self.CloseConversation`))))
            (:`1`
              (bind _state_3 (`self.AddDialogue` (`self.Character Name`) "Okay we make home!" (`|MakeArray` "Continue" :!type "Text")))
              (switch `/Game/Goobin/Dialogue/E_DialogueState` _state_3
                (:`NewEnumerator0`
                  (bind _isable (`/Game/Goobin/Blueprints/BP_Village.CheckIfAble` _village (`|MakeArray` "Wood" "Rock" :!type "Name") (`|MakeArray` 2 1)))
                  (if _isable
                    (`/Game/Goobin/Blueprints/BP_Village.CreateBuilding` _village "Test")
                    (`self.ClearDialogueProgress`)
                    (`self.CloseConversation`)
                    (else
                      (bind _state_4 (`self.AddDialogue` (`self.Character Name`) "You no have things to make!" (`|MakeArray` "Continue" :!type "Text")))
                      (switch `/Game/Goobin/Dialogue/E_DialogueState` _state_4
                        (:`NewEnumerator0`
                          (`self.ClearDialogueProgress`)
                          (`self.CloseConversation`))))))))))))
    (:`1`
      (bind _state_5 (`self.AddDialogue` (`self.Character Name`) "Go way! Still not talking!" (`|MakeArray` "Grrr" "What be evers" :!type "Text")))
      (switch `/Game/Goobin/Dialogue/E_DialogueState` _state_5
        (:`NewEnumerator0`
          (`self.ClearDialogueProgress`)
          (`self.CloseConversation`))))))