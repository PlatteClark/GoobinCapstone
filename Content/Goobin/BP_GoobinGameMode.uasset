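; Game mode that persists per-level actor changes through a SaveData_Level save slot named after the current level.
; On BeginPlay it loads or creates that save, spawns the ActorsAdded classes at their stored transforms and destroys any valid ActorsRemoved actors.
; It writes the save to the slot right after loading or creating it, and again on EndPlay.
; The added and removed records are only read here.
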(event `self.ReceiveBeginPlay`
  (bind _as_save_data_level (`self.As Save Data Level`))
  (bind _actorsadded (`/Game/Goobin/Save/SaveData_Level.ActorsAdded` _as_save_data_level))
  (bind _returnvalue (`GameplayStatics.GetCurrentLevelName` true))
  (bind _output_get (set `self.LevelDataSlot` (`KismetStringLibrary.Concat_StrStr` _returnvalue "_Data")))
  (bind _returnvalue_2 (`GameplayStatics.DoesSaveGameExist` _output_get))
  (if _returnvalue_2
    (bind _returnvalue_3 (`GameplayStatics.LoadGameFromSlot` (`self.LevelDataSlot`)))
    (bind _assave_data_level (cast `/Game/Goobin/Save/SaveData_Level` _returnvalue_3))
    (bind _output_get_2 (set `self.As Save Data Level` _assave_data_level))
    (`GameplayStatics.SaveGameToSlot` _output_get_2 (`self.LevelDataSlot`))
    (bind _keys (`BlueprintMapLibrary.Map_Keys` _actorsadded))
    (for _array_element _keys
      (`|SpawnActorFromClass` (`|ConvertAsset` _array_element) (`BlueprintMapLibrary.Map_Find` _actorsadded _array_element) "AlwaysSpawn" "MultiplyWithRoot" null null))
    (for _array_element_2 (`/Game/Goobin/Save/SaveData_Level.ActorsRemoved` _as_save_data_level)
      (bind _output (`|ConvertAsset` _array_element_2))
      (`/Engine/EditorBlueprintResources/StandardMacros.IsValid` _output
        (:`Is Valid`
          (`self.K2_DestroyActor` _output))))
    (else
      (bind _returnvalue_4 (`GameplayStatics.CreateSaveGameObject` "/Game/Goobin/Save/SaveData_Level.SaveData_Level_C"))
      (bind _output_get_3 (set `self.As Save Data Level` _returnvalue_4))
      (`GameplayStatics.SaveGameToSlot` _output_get_3 (`self.LevelDataSlot`)))))

(event `self.ReceiveEndPlay`
  (params (EndPlayReason :type "EEndPlayReason Enum" :default "Destroyed"))
  (`GameplayStatics.SaveGameToSlot` (`self.As Save Data Level`) (`self.LevelDataSlot`)))

(fn `UserConstructionScript`)