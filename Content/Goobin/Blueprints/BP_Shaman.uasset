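; Shaman NPC, the village leader who gives the tutorial and fruit quest, then serves as the player's goobin command menu.
; DialogueTree branches on the dialogue component's DialogueTreeIndex, advancing as quest stages complete.
; Accepting chores enables collision on the held axe; turning in fruit checks inventory, takes it and spawns a goobin.
; Later menu choices call SpawnGoobin or CallToWar on the BP_Village found at BeginPlay, with no item cost here.
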(event `self.ReceiveBeginPlay`
  (`parent.ReceiveBeginPlay`)
  (bind _returnvalue (`GameplayStatics.GetActorOfClass` "/Game/Goobin/Blueprints/BP_Village.BP_Village_C"))
  (set `self.Village` _returnvalue))

(fn `Dialogue Tree`
  (bind _village (`self.Village`))
  (switch `int` (`/Game/Goobin/Dialogue/AC_DialogueBase.DialogueTreeIndex` (`self.AC_DialogueBase`))
    (:`Default`
      (bind (_state _optionindex) (`/Game/Goobin/Dialogue/AC_DialogueBase.AddDialogue` (`self.AC_DialogueBase`) (`self.CharacterName`) "Shaman hear you. What want?" (`|MakeArray` "Make a Goobin." "I want goobins to follow me!" :!type "Text") :!label _label))
      (switch `/Game/Goobin/Dialogue/E_DialogueState` _state
        (:`NewEnumerator0`
          (switch `int` _optionindex
            (:`0`
              (`/Game/Goobin/Blueprints/BP_Village.SpawnGoobin` _village))
            (:`1`
              (`/Game/Goobin/Blueprints/BP_Village.CallToWar` _village)))
          (`/Game/Goobin/Dialogue/AC_DialogueBase.ClearDialogueProgress` (`self.AC_DialogueBase`))
          (`/Game/Goobin/Dialogue/AC_DialogueBase.CloseConversation` (`self.AC_DialogueBase`)))))
    (:`0`
      ;[0 0.2604 0.002974] Tutorial
      (bind (_state_2 _optionindex_2) (`/Game/Goobin/Dialogue/AC_DialogueBase.AddDialogue` (`self.AC_DialogueBase`) (`self.CharacterName`) "Hello young goob, and welcome to the world! I the Shaman! I am leader of village! " (`|MakeArray` "How do I do things?" "I no know what to do..." :!type "Text")))
      (switch `/Game/Goobin/Dialogue/E_DialogueState` _state_2
        (:`NewEnumerator0`
          (switch `int` _optionindex_2
            (:`0`
              (bind (_state_3 _optionindex_3) (`/Game/Goobin/Dialogue/AC_DialogueBase.AddDialogue` (`self.AC_DialogueBase`) (`self.CharacterName`) "I guess we have another dumb goobin... You interact with things by pressing \"e\", open your inventory with \"i\", and equiping things by dragging onto your body in the top left corner." (`|MakeArray` "Oh... I guess that makes sense..." "Wait! That was a lot of things! Again please!" :!type "Text") :!label _label_2))
              (switch `/Game/Goobin/Dialogue/E_DialogueState` _state_3
                (:`NewEnumerator0`
                  (switch `int` _optionindex_3
                    (:`0`
                      (bind (_state_4 _optionindex_4) (`/Game/Goobin/Dialogue/AC_DialogueBase.AddDialogue` (`self.AC_DialogueBase`) (`self.CharacterName`) "Good... good. Maybe yous not as slow as me thinks before. Okay, well... Go work now." (`|MakeArray` "Work? I don't know what to do..." "(Lie) Oh yes, of course! very busys! Will go work for sure. No needing to check on me. I very worker!" :!type "Text")))
                      (switch `/Game/Goobin/Dialogue/E_DialogueState` _state_4
                        (:`NewEnumerator0`
                          (switch `int` _optionindex_4
                            (:`0`
                              (bind (_state_5 _optionindex_5) (`/Game/Goobin/Dialogue/AC_DialogueBase.AddDialogue` (`self.AC_DialogueBase`) (`self.CharacterName`) "Well, to start, take my old axe, it not too good no more. Bring me 5 fruits from that green tree in the center, we need them to raise more goobins to fight yellow tribe." (`|MakeArray` "CHORES?! NOOO!!" "The yellow tribe...?" :!type "Text") :!label _label_3))
                              (switch `/Game/Goobin/Dialogue/E_DialogueState` _state_5
                                (:`NewEnumerator0`
                                  (switch `int` _optionindex_5
                                    (:`0`
                                      _)
                                    (:`1`
                                      (bind (_state_6 _optionindex_6) (`/Game/Goobin/Dialogue/AC_DialogueBase.AddDialogue` (`self.AC_DialogueBase`) (`self.CharacterName`) "Yeah the yellow tribe has made life hard for us green tribe. They get all the best foods up by the lake, and still them comes and takes our foods sometimes! Not good! So we fight back now!" (`|MakeArray` "I still don't want to do chores, though..." "Maybe I join yellow tribe because they don't make me do chores!" :!type "Text")))
                                      (switch `/Game/Goobin/Dialogue/E_DialogueState` _state_6
                                        (:`NewEnumerator0`
                                          (switch `int` _optionindex_6
                                            (:`0`
                                              _)
                                            (:`1`
                                              _))))))
                                  (bind (_state_7 _optionindex_7) (`/Game/Goobin/Dialogue/AC_DialogueBase.AddDialogue` (`self.AC_DialogueBase`) (`self.CharacterName`) "Now now, chores is good for a young goobin! Makes you grow strong, or something. And we kick you out of tribe if you don't work. You can have the axe in my hand now." (`|MakeArray` "I wish I didn't get out of bed..." "I go collect things for you." :!type "Text")))
                                  (switch `/Game/Goobin/Dialogue/E_DialogueState` _state_7
                                    (:`NewEnumerator0`
                                      (switch `int` _optionindex_7
                                        (:`Default`
                                          _)
                                        (:`0`
                                          _)
                                        (:`1`
                                          _))
                                      (`self.SetActorEnableCollision` (`ChildActorComponent.ChildActor` (`self.LeftHand`)) true)
                                      (`/Game/Goobin/Dialogue/AC_DialogueBase.ClearDialogueProgress` (`self.AC_DialogueBase`))
                                      (`/Game/Goobin/Dialogue/AC_DialogueBase.CloseConversation` (`self.AC_DialogueBase`))
                                      (set `/Game/Goobin/Dialogue/AC_DialogueBase.DialogueTreeIndex` 1 (`self.AC_DialogueBase`)))))))
                            (:`1`
                              (bind (_state_8 _optionindex_8) (`/Game/Goobin/Dialogue/AC_DialogueBase.AddDialogue` (`self.AC_DialogueBase`) (`self.CharacterName`) "Hmm. Shaman really want to believe you, since it been so long since another goobin love work. FINE! I believes." (`|MakeArray` "Hehe... Shamans no is smarts! Now I go play!" :!type "Text")))
                              (switch `/Game/Goobin/Dialogue/E_DialogueState` _state_8
                                (:`NewEnumerator0`
                                  (switch `int` _optionindex_8
                                    (:`Default`
                                      _)
                                    (:`0`
                                      _))
                                  (`/Game/Goobin/Dialogue/AC_DialogueBase.ClearDialogueProgress` (`self.AC_DialogueBase`))
                                  (`/Game/Goobin/Dialogue/AC_DialogueBase.CloseConversation` (`self.AC_DialogueBase`)))))))))
                    (:`1`
                      (goto _label_2))))))
            (:`1`
              (goto _label_3))))))
    (:`1`
      (bind (_state_9 _optionindex_9) (`/Game/Goobin/Dialogue/AC_DialogueBase.AddDialogue` (`self.AC_DialogueBase`) (`self.CharacterName`) "Did you bring me the food yet?" (`|MakeArray` "Yes!" "...No getting food is hard!" :!type "Text")))
      (switch `/Game/Goobin/Dialogue/E_DialogueState` _state_9
        (:`NewEnumerator0`
          (switch `int` _optionindex_9
            (:`0`
              (if (`/Game/Goobin/Inventory/AC_InventorySystem.QueryInventory` (`/Game/Goobin/Blueprints/BP_Character.AC_Inventory` (cast `/Game/Goobin/Blueprints/BP_Character` (`self.InteractInstigator`) :!pure true)) "Fruit" 5)
                (bind (_state_10 _optionindex_10) (`/Game/Goobin/Dialogue/AC_DialogueBase.AddDialogue` (`self.AC_DialogueBase`) (`self.CharacterName`) "GOOD! We make goobin now! We need to fight the yellow tribe up by the lake! They have taken the food and water suply, which we desperately need back! Raise MORE goobin! Go fight! (Recommended 10 goobs to fight yellow tribe) YOU MUST DESTROY THEIR TOTEM TO DESTROY THEM!!" (`|MakeArray` "Okay" :!type "Text")))
                (switch `/Game/Goobin/Dialogue/E_DialogueState` _state_10
                  (:`NewEnumerator0`
                    (switch `int` _optionindex_10
                      (:`Default`
                        _)
                      (:`0`
                        _))
                    (`self.TakeItemsFromPlayer` "Fruit" 5)
                    (`/Game/Goobin/Blueprints/BP_Village.SpawnGoobin` (`self.Village`))
                    (`/Game/Goobin/Dialogue/AC_DialogueBase.ClearDialogueProgress` (`self.AC_DialogueBase`))
                    (`/Game/Goobin/Dialogue/AC_DialogueBase.CloseConversation` (`self.AC_DialogueBase`))
                    (set `/Game/Goobin/Dialogue/AC_DialogueBase.DialogueTreeIndex` 2 (`self.AC_DialogueBase`))))
                (else
                  (bind (_state_11 _optionindex_11) (`/Game/Goobin/Dialogue/AC_DialogueBase.AddDialogue` (`self.AC_DialogueBase`) (`self.CharacterName`) "YOU dumb and bad goobin! Bring me 5 fruits from the tree in the middle of town! Is not that hard!" (`|MakeArray` "Okay" :!type "Text")))
                  (switch `/Game/Goobin/Dialogue/E_DialogueState` _state_11
                    (:`NewEnumerator0`
                      (switch `int` _optionindex_11
                        (:`Default`
                          _)
                        (:`0`
                          _))
                      (`/Game/Goobin/Dialogue/AC_DialogueBase.ClearDialogueProgress` (`self.AC_DialogueBase`))
                      (`/Game/Goobin/Dialogue/AC_DialogueBase.CloseConversation` (`self.AC_DialogueBase`)))))))))))
    (:`2`
      (goto _label))))

(fn `UserConstructionScript`
  (`parent.UserConstructionScript`))