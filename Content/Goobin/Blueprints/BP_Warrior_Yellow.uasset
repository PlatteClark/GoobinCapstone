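; Yellow-team AI warrior character that fights with a bone spear and can be looted once dead.
; On BeginPlay it spawns and attaches the spear to its hand, starts its behavior tree and seeds its inventory with the spear and random coins.
; Cover, Advance, Retreat and Attack events drive crouching and a montage-based thrust that toggles the weapon active, then reports noise.
; Hits report touch to AI perception; interacting at zero health opens its inventory.
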(event `self.ReceiveBeginPlay`
  (bind _returnvalue (`|SpawnActorFromClass` "/Game/Goobin/Inventory/Items/Weapons/BP_BoneSpear.BP_BoneSpear_C" (`KismetMathLibrary.MakeTransform` (0.0 0.0 0.0)) "Undefined" "MultiplyWithRoot" null null))
  (`/Engine/EditorBlueprintResources/StandardMacros.IsValid` _returnvalue
    (:`Is Valid`
      (set `self.HeldWeapon` _returnvalue)
      (set `/Game/Goobin/Inventory/Items/Weapons/BP_BoneSpear.OwnerTag` "Yellow" _returnvalue)
      (bind _returnvalue_2 (`self.GetComponentByClass` _returnvalue "/Script/Engine.StaticMeshComponent"))
      (`PrimitiveComponent.SetSimulatePhysics` _returnvalue_2 false)
      (`PrimitiveComponent.SetCollisionResponseToChannel` _returnvalue_2 "ECC_GameTraceChannel1" "ECR_Ignore")
      (`self.K2_AttachToComponent` _returnvalue (`self.Mesh`) "Socket_Hand.R" "SnapToTarget" "SnapToTarget" "SnapToTarget" true)
      (`AIController.RunBehaviorTree` (`AIBlueprintHelperLibrary.GetAIController` self) "/Game/Goobin/AI/Yellow/BT_Warrior_Yellow.BT_Warrior_Yellow")
      (if (not (`/Game/Goobin/Inventory/AC_InventorySystem.QueryInventory` (`self.AC_InventorySystem`) "BoneSpear" 1))
        (`/Game/Goobin/Inventory/AC_InventorySystem.AddToInventory` (`self.AC_InventorySystem`) "BoneSpear" 1)
        (`/Game/Goobin/Inventory/AC_InventorySystem.AddToInventory` (`self.AC_InventorySystem`) "Coin" (`KismetMathLibrary.RandomIntegerInRange` 1 10))))))

(event `self.ReceiveHit`
  (params (MyComp :type "PrimitiveComponent Object Reference") (Other :type "Actor Object Reference") (OtherComp :type "PrimitiveComponent Object Reference") (bSelfMoved :type Boolean) (HitLocation :type "Vector Structure") (HitNormal :type "Vector Structure") (NormalImpulse :type "Vector Structure") (Hit :type "HitResult Structure (by ref)"))
  (`AISense_Touch.ReportTouchEvent` self Other HitLocation))

(event `self.SetInteractableState`
  (params (IsVisible :type Boolean))
  (bind _txt_charactername (`self.Txt_CharacterName`))
  (if IsVisible
    (`SceneComponent.SetVisibility` _txt_charactername true false)
    (else
      (`SceneComponent.SetVisibility` _txt_charactername false false))))

(event `self.ConversationClosed`
  (message `/Game/Goobin/Blueprints/BPI_Interactable.ConversationClosed` (`self.InteractInstigator`)))

(event `self.Cover`
  (`self.Crouch`))

(event `self.Advance`
  (`self.UnCrouch`))

(event `self.Retreat`
  (`self.UnCrouch`))

(event `self.Attack`
  (`self.UnCrouch`)
  (set `/Game/Goobin/Inventory/Items/Weapons/BP_BoneSpear.IsActive` true (`self.HeldWeapon`))
  (bind _returnvalue (`self.PlayAnimMontage` "/Game/Goobin/Animations/Goobin/AM_SpearThrust.AM_SpearThrust" 0.7))
  (`KismetSystemLibrary.Delay` _returnvalue)
  (set `/Game/Goobin/Inventory/Items/Weapons/BP_BoneSpear.IsActive` false (`self.HeldWeapon`))
  (`AISense_Hearing.ReportNoiseEvent` (`self.K2_GetActorLocation`) 300.0 self))

(event `self.Interact`
  (params (Instigator :type "Actor Object Reference"))
  (if (not (> (`self.Health`) 0.0))
    (bind _asplayer_controller_goobin (cast `/Game/Goobin/Blueprints/PlayerController_Goobin` (`GameplayStatics.GetPlayerController` 0)))
    (`/Game/Goobin/UI/W_HUD.ShowContainer` (`/Game/Goobin/Blueprints/PlayerController_Goobin.HUD` _asplayer_controller_goobin) (`self.AC_InventorySystem`))))

(fn `DropLoot`
  (`parent.DropLoot`)
  (`self.K2_DestroyActor` (`self.HeldWeapon`)))

(fn `UserConstructionScript`
  (`parent.UserConstructionScript`))