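; NPC shopkeeper that sells a bone spear to the player for wood through a branching conversation.
; The Dialogue Tree chains ACDialogueBase nodes by option index, and both payment replies, honest or lying, run the same inventory check on the interacting BP_Character.
; On success it takes the wood through the parent's TakeItemsFromPlayer and spawns BP_BoneSpear at SpawnTransform.
; Each ending clears dialogue progress and closes the conversation.
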(fn `Dialogue Tree`
  (bind _ac_dialoguebase (`self.AC_DialogueBase`))
  (bind _ac_dialoguebase_2 (`self.AC_DialogueBase`))
  (bind _ac_dialoguebase_3 (`self.AC_DialogueBase`))
  (bind (_state _optionindex) (`/Game/Goobin/Dialogue/AC_DialogueBase.AddDialogue` (`self.AC_DialogueBase`) (`self.CharacterName`) "You want bone Spear?" (`|MakeArray` "OH YES!" "Nah I like to use hands." :!type "Text")))
  (switch `/Game/Goobin/Dialogue/E_DialogueState` _state
    (:`NewEnumerator0`
      (switch `int` _optionindex
        (:`0`
          (bind (_state_2 _optionindex_2) (`/Game/Goobin/Dialogue/AC_DialogueBase.AddDialogue` (`self.AC_DialogueBase`) (`self.CharacterName`) "YAY! It cost 2 wood." (`|MakeArray` "I have the wood." "(Lie) I have the wood." :!type "Text")))
          (switch `/Game/Goobin/Dialogue/E_DialogueState` _state_2
            (:`NewEnumerator0`
              (switch `int` _optionindex_2
                (:`0`
                  _)
                (:`1`
                  _))
              (if (`/Game/Goobin/Inventory/AC_InventorySystem.QueryInventory` (`/Game/Goobin/Blueprints/BP_Character.AC_Inventory` (cast `/Game/Goobin/Blueprints/BP_Character` (`self.InteractInstigator`) :!pure true)) "Wood" 2)
                (bind (_state_3 _optionindex_3) (`/Game/Goobin/Dialogue/AC_DialogueBase.AddDialogue` (`self.AC_DialogueBase`) (`self.CharacterName`) "Is good wood! Here go!" (`|MakeArray` "Thanks, Bone-Pounder." "Hope it was worth it." :!type "Text")))
                (switch `/Game/Goobin/Dialogue/E_DialogueState` _state_3
                  (:`NewEnumerator0`
                    (switch `int` _optionindex_3
                      (:`0`
                        _)
                      (:`1`
                        _))
                    (`/Game/Goobin/Dialogue/AC_DialogueBase.ClearDialogueProgress` _ac_dialoguebase)
                    (`self.TakeItemsFromPlayer` "Wood" 2)
                    (`|SpawnActorFromClass` "/Game/Goobin/Inventory/Items/Weapons/BP_BoneSpear.BP_BoneSpear_C" (`SceneComponent.K2_GetComponentToWorld` (`self.Spawn Transform`)) "AlwaysSpawn" "MultiplyWithRoot" null null)
                    (`/Game/Goobin/Dialogue/AC_DialogueBase.CloseConversation` _ac_dialoguebase)))
                (else
                  (bind (_state_4 _optionindex_4) (`/Game/Goobin/Dialogue/AC_DialogueBase.AddDialogue` (`self.AC_DialogueBase`) (`self.CharacterName`) "Lies! You no have wood!" (`|MakeArray` "I am not a smart goobin." "What is wood?" :!type "Text")))
                  (switch `/Game/Goobin/Dialogue/E_DialogueState` _state_4
                    (:`NewEnumerator0`
                      (switch `int` _optionindex_4
                        (:`0`
                          _)
                        (:`1`
                          _))
                      (`/Game/Goobin/Dialogue/AC_DialogueBase.ClearDialogueProgress` _ac_dialoguebase_3)
                      (`/Game/Goobin/Dialogue/AC_DialogueBase.CloseConversation` _ac_dialoguebase_3))))))))
        (:`1`
          (bind (_state_5 _optionindex_5) (`/Game/Goobin/Dialogue/AC_DialogueBase.AddDialogue` (`self.AC_DialogueBase`) (`self.CharacterName`) "Some day someone will buy one..." (`|MakeArray` "Is not today." "If you thinks." :!type "Text")))
          (switch `/Game/Goobin/Dialogue/E_DialogueState` _state_5
            (:`NewEnumerator0`
              (switch `int` _optionindex_5
                (:`0`
                  _)
                (:`1`
                  _))
              (`/Game/Goobin/Dialogue/AC_DialogueBase.ClearDialogueProgress` _ac_dialoguebase_2)
              (`/Game/Goobin/Dialogue/AC_DialogueBase.CloseConversation` _ac_dialoguebase_2))))))))

(fn `TakeItemsFromPlayer`
  (params (ItemID :type Name) (Quantity :type Integer))
  (returns (Successful :type Boolean))
  (bind _successful (`parent.TakeItemsFromPlayer` ItemID Quantity))
  (return _successful))

(fn `UserConstructionScript`
  (`parent.UserConstructionScript`))