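; BP_Village is a village actor that spawns buildings and handles their item costs from the player's inventory.
; CreateBuilding maps a building name to a spawn, currently only a Test case placing BP_GoobinHut at HutSpawn.
; Separately, CheckIfAble verifies quantities in BP_Character's inventory, then deducts them through RemoveFromInventory one unit at a time.
; Construction hides the built-in hut meshes; the logic to reveal them is disconnected.
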(event `self.ReceiveBeginPlay`
  (bind _returnvalue (`GameplayStatics.GetActorOfClass` "/Game/Goobin/Blueprints/BP_Character.BP_Character_C"))
  (set `self.Player` _returnvalue))

(event `CreateBuilding`
  (params (`Building Name` :type Name))
  (switch `name` `Building Name`
    (:`Test`
      (`|SpawnActorFromClass` "/Game/Goobin/Blueprints/Buildings/BP_GoobinHut.BP_GoobinHut_C" (`SceneComponent.K2_GetComponentToWorld` (`self.HutSpawn`)) "AdjustIfPossibleButAlwaysSpawn" "MultiplyWithRoot" null null))))

(fn `CheckIfAble`
  (params (Names :type "Array of Name") (Costs :type "Array of Integer"))
  (returns (IsAble :type Boolean))
  (locals (LocalCost :type Integer) (LocalIndex :type Integer :default 0))
  (bind _ac_inventory (`/Game/Goobin/Blueprints/BP_Character.AC_Inventory` (`self.Player`)))
  (for (_array_element _array_index) Names
    (bind (_index _foundslot) (`/Game/Goobin/Inventory/AC_InventorySystem.FindSlot` _ac_inventory _array_element))
    (if _foundslot
      (set `local.LocalCost` (`|GetArrayItem` Costs _array_index))
      (if (not (>= (`.Quantity_5_F87394DD4E2C0007D65DFB9D51E10CB1` (break `/Game/Goobin/Inventory/FSlotStruct` (`|GetArrayItem` (`/Game/Goobin/Inventory/AC_InventorySystem.Content` _ac_inventory) _index))) (`local.LocalCost`)))
        (return false))
      (else
        (return false))))
  (`self.RemoveFromInventory` (`local.Names`) (`local.Costs`))
  (return true))

(fn `RemoveFromInventory`
  (params (Names :type "Array of Name") (Costs :type "Array of Integer"))
  (bind _ac_inventory (`/Game/Goobin/Blueprints/BP_Character.AC_Inventory` (`self.Player`)))
  (for (_array_element _array_index) Names
    (for _ (range 1 (+ (`|GetArrayItem` Costs _array_index) 1))
      (bind (_index _foundslot) (`/Game/Goobin/Inventory/AC_InventorySystem.FindSlot` _ac_inventory _array_element))
      (if _foundslot
        (`/Game/Goobin/Inventory/AC_InventorySystem.RemoveFromInventory` _ac_inventory _index false true)))))

(fn `UserConstructionScript`
  (bind _goobinhut_hut_base (`self.GoobinHut_Hut_Base`))
  (`SceneComponent.SetVisibility` _goobinhut_hut_base false false)
  (`SceneComponent.SetVisibility` (`self.GoobinHut_Rocks`) false false)
  (`PrimitiveComponent.SetCollisionEnabled` _goobinhut_hut_base "NoCollision"))