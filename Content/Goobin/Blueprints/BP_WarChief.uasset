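; BP_WarChief is a war chief NPC that invites the player to war through a branching conversation.
; Its DialogueTree switches on the dialogue component's tree index and offers a yes or no choice through AddDialogue, continuing on the Pass Through state.
; Accepting opens the Arena level, while refusing shows a dismissive reply; both branches then clear dialogue progress and close the conversation.
; The event graph holds only disabled default events.
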(fn `Dialogue Tree`
  (bind _ac_dialoguebase (`self.AC_DialogueBase`))
  (bind _ac_dialoguebase_2 (`self.AC_DialogueBase`))
  (switch `int` (`/Game/Goobin/Dialogue/AC_DialogueBase.DialogueTreeIndex` (`self.AC_DialogueBase`))
    (:`0`
      (bind (_state _optionindex) (`/Game/Goobin/Dialogue/AC_DialogueBase.AddDialogue` (`self.AC_DialogueBase`) (`self.CharacterName`) "Hi fellow! Want to war?" (`|MakeArray` "Yes! I love war!" "No, I want peace." :!type "Text")))
      (switch `/Game/Goobin/Dialogue/E_DialogueState` _state
        (:`NewEnumerator0`
          (switch `int` _optionindex
            (:`0`
              (`GameplayStatics.OpenLevel` "Arena")
              (`/Game/Goobin/Dialogue/AC_DialogueBase.ClearDialogueProgress` _ac_dialoguebase)
              (`/Game/Goobin/Dialogue/AC_DialogueBase.CloseConversation` _ac_dialoguebase))
            (:`1`
              (bind _state_2 (`/Game/Goobin/Dialogue/AC_DialogueBase.AddDialogue` (`self.AC_DialogueBase`) (`self.CharacterName`) "Gah! This Goobin is no war-fighter. Come back when strong!" (`|MakeArray` "Continue" :!type "Text")))
              (switch `/Game/Goobin/Dialogue/E_DialogueState` _state_2
                (:`NewEnumerator0`
                  (`/Game/Goobin/Dialogue/AC_DialogueBase.ClearDialogueProgress` _ac_dialoguebase_2)
                  (`/Game/Goobin/Dialogue/AC_DialogueBase.CloseConversation` _ac_dialoguebase_2))))))))))

(fn `UserConstructionScript`
  (`parent.UserConstructionScript`))