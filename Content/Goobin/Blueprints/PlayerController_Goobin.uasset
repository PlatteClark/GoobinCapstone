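; Player controller for the Goobin game that owns the player's HUD widget.
; On BeginPlay for the local controller it creates a W_HUD widget and adds it to the viewport.
; ResetHUD removes the current HUD, prints a debug string and rebuilds it through the same creation path.
; The IA_Inventory input action tells the HUD to display the player menu.
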(event `ResetHUD`
  (`Widget.RemoveFromParent` (`self.HUD`))
  (`KismetSystemLibrary.PrintString` "Hello")
  (bind _returnvalue (`|CreateWidget` "/Game/Goobin/UI/W_HUD.W_HUD_C" :!label _label))
  (bind _output_get (set `self.HUD` _returnvalue))
  (`UserWidget.AddToViewport` _output_get 0))

(event `self.ReceiveBeginPlay`
  (if (`self.IsLocalPlayerController`)
    (goto _label)))

(event `EnhancedInput|/Game/Goobin/Input/Actions/IA_Inventory`
  (params (ActionValue :type Boolean) (ElapsedSeconds :type "Float (double-precision)") (TriggeredSeconds :type "Float (double-precision)") (InputAction :type "InputAction Object Reference" :default "/Game/Goobin/Input/Actions/IA_Inventory.IA_Inventory"))
  (:`Triggered`
    (`/Game/Goobin/UI/W_HUD.DisplayPlayerMenu` (`self.HUD`))))

(fn `UserConstructionScript`)