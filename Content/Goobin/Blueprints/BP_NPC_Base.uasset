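; Base NPC Blueprint with a name label, interaction and conversation hooks, and a ragdoll reaction to damage.
; The construction script fills the label from CharacterName, and SetInteractableState toggles its visibility.
; ConversationClosed relays a closed message to the interaction instigator, while LookAt returns an empty string.
; Any damage, regardless of amount, switches the mesh to physics simulation with the Ragdoll collision profile.
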(event `/Game/Goobin/Blueprints/BPI_Interactable.SetInteractableState`
  (params (IsVisible :type Boolean))
  (bind _txt_charactername (`self.Txt_CharacterName`))
  (if IsVisible
    (`SceneComponent.SetVisibility` _txt_charactername true false)
    (else
      (`SceneComponent.SetVisibility` _txt_charactername false false))))

(event `/Game/Goobin/Blueprints/BPI_Interactable.ConversationClosed`
  (message `/Game/Goobin/Blueprints/BPI_Interactable.ConversationClosed` (`self.InteractInstigator`)))

(event `self.ReceiveAnyDamage`
  (params (Damage :type "Float (single-precision)") (DamageType :type "DamageType Object Reference") (InstigatedBy :type "Controller Object Reference") (DamageCauser :type "Actor Object Reference"))
  (bind _mesh (`self.Mesh`))
  (`PrimitiveComponent.SetSimulatePhysics` _mesh true)
  (`PrimitiveComponent.SetCollisionProfileName` _mesh "Ragdoll" true))

(fn `LookAt`
  (returns (Message :type Text))
  (return ""))

(fn `UserConstructionScript`
  (`TextRenderComponent.K2_SetText` (`self.Txt_CharacterName`) (`self.CharacterName`)))