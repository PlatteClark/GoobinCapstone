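; BP_Archer_Yellow is an AI archer character that fights with a wooden bow and can be looted once dead.
; On BeginPlay it attaches a spawned bow to its hand, runs its behavior tree and stocks its inventory with the bow and random coins.
; Cover, Advance, Retreat and Attack events set crouch state, with Attack using the held bow.
; Hits report touch to AI perception; an older arrow-firing chain is left unconnected.
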(event `self.ReceiveBeginPlay`
  (`self.UnCrouch`)
  (bind _returnvalue (`|SpawnActorFromClass` "/Game/Goobin/Inventory/Items/Weapons/BP_WoodBow.BP_WoodBow_C" (`KismetMathLibrary.MakeTransform` (0.0 0.0 0.0)) "Undefined" "MultiplyWithRoot" null null))
  (`/Engine/EditorBlueprintResources/StandardMacros.IsValid` _returnvalue
    (:`Is Valid`
      (set `self.HeldWeapon` _returnvalue)
      (bind _returnvalue_2 (`self.GetComponentByClass` _returnvalue "/Script/Engine.StaticMeshComponent"))
      (`PrimitiveComponent.SetSimulatePhysics` _returnvalue_2 false)
      (`PrimitiveComponent.SetCollisionResponseToChannel` _returnvalue_2 "ECC_GameTraceChannel1" "ECR_Ignore")
      (`self.K2_AttachToComponent` _returnvalue (`self.Mesh`) "Socket_Hand.L" "SnapToTarget" "SnapToTarget" "SnapToTarget" true)
      (`AIController.RunBehaviorTree` (`AIBlueprintHelperLibrary.GetAIController` self) "/Game/Goobin/AI/Yellow/BT_Archer_Yellow_New.BT_Archer_Yellow_New")
      (if (not (`/Game/Goobin/Inventory/AC_InventorySystem.QueryInventory` (`self.AC_InventorySystem`) "WoodBow" 1))
        (`/Game/Goobin/Inventory/AC_InventorySystem.AddToInventory` (`self.AC_InventorySystem`) "WoodBow" 1)
        (`/Game/Goobin/Inventory/AC_InventorySystem.AddToInventory` (`self.AC_InventorySystem`) "Coin" (`KismetMathLibrary.RandomIntegerInRange` 1 10))))))

(event `self.ReceiveHit`
  (params (MyComp :type "PrimitiveComponent Object Reference") (Other :type "Actor Object Reference") (OtherComp :type "PrimitiveComponent Object Reference") (bSelfMoved :type Boolean) (HitLocation :type "Vector Structure") (HitNormal :type "Vector Structure") (NormalImpulse :type "Vector Structure") (Hit :type "HitResult Structure (by ref)"))
  (`AISense_Touch.ReportTouchEvent` self Other HitLocation))

(event `/Game/Goobin/Blueprints/BPI_Interactable.SetInteractableState`
  (params (IsVisible :type Boolean))
  (bind _txt_charactername (`self.Txt_CharacterName`))
  (if IsVisible
    (`SceneComponent.SetVisibility` _txt_charactername true false)
    (else
      (`SceneComponent.SetVisibility` _txt_charactername false false))))

(event `/Game/Goobin/Blueprints/BPI_Interactable.ConversationClosed`
  (message `/Game/Goobin/Blueprints/BPI_Interactable.ConversationClosed` (`self.InteractInstigator`)))

(event `/Game/Goobin/AI/BPI_Combat.Cover`
  (`self.Crouch`))

(event `/Game/Goobin/AI/BPI_Combat.Advance`
  (`self.UnCrouch`))

(event `/Game/Goobin/AI/BPI_Combat.Retreat`
  (`self.UnCrouch`))

(event `/Game/Goobin/AI/BPI_Combat.Attack`
  (`self.UnCrouch`)
  (`/Game/Goobin/Blueprints/BPI_Interactable.UseItem` (`self.HeldWeapon`) self))

(event `/Game/Goobin/Blueprints/BPI_Interactable.Interact`
  (params (Instigator :type "Actor Object Reference"))
  (if (not (> (`self.Health`) 0.0))
    (bind _asplayer_controller_goobin (cast `/Game/Goobin/Blueprints/PlayerController_Goobin` (`GameplayStatics.GetPlayerController` 0)))
    (`/Game/Goobin/UI/W_HUD.ShowContainer` (`/Game/Goobin/Blueprints/PlayerController_Goobin.HUD` _asplayer_controller_goobin) (`self.AC_InventorySystem`))))

(fn `DropLoot`
  (`parent.DropLoot`)
  (`self.K2_DestroyActor` (`self.HeldWeapon`)))

(fn `UserConstructionScript`
  (`parent.UserConstructionScript`))