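; BP_NPC_Test is a test NPC that players can talk to through an ACDialogueNPCTest dialogue component.
; Interacting stores the instigator, toggles their movement and opens the conversation; closing it toggles movement again, notifies the instigator and plays a sound at world origin.
; The construction script copies CharacterName into the component, and LookAt returns a "Talk to {Name}" prompt built from that name.
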(event `self.Interact`
  (params (Instigator :type "Actor Object Reference"))
  (bind _output_get (set `self.InteractInstigator` Instigator))
  (`/Game/Goobin/Dialogue/AC_DialogueBase.TogglePlayerMovement` (`self.AC_Dialogue_NPC_Test`) _output_get)
  (`/Game/Goobin/Dialogue/AC_DialogueBase.OpenConversation` (`self.AC_Dialogue_NPC_Test`)))

(event `self.ConversationClosed`
  (`/Game/Goobin/Dialogue/AC_DialogueBase.TogglePlayerMovement` (`self.AC_Dialogue_NPC_Test`) (`self.InteractInstigator`))
  (message `/Game/Goobin/Blueprints/BPI_Interactable.ConversationClosed` (`self.InteractInstigator`))
  (`GameplayStatics.PlaySoundAtLocation` "/Engine/EditorSounds/Notifications/CompileStart_Cue.CompileStart_Cue" (0.0 0.0 0.0) (struct) 1.0 1.0 0.0 null null null null))

(fn `LookAt`
  (returns (Message :type Text))
  (return (`|FormatText` "Talk to {Name}" (`self.CharacterName`))))

(fn `UserConstructionScript`
  (`parent.UserConstructionScript`)
  (set `/Game/Goobin/Dialogue/AC_Dialogue_NPC_Test.Character Name` (`self.CharacterName`) (`self.AC_Dialogue_NPC_Test`)))