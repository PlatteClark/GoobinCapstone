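; BP_Fire is an environmental fire hazard that deals damage and casts a flickering light.
; A fast looping timer started on BeginPlay randomizes the point light's intensity within a clamped range.
; Actors that begin overlapping its sphere take a small one-off hit of damage.
; Disconnected nodes that would spawn another BP_Fire attached to the overlapping actor never run.
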(event `self.ReceiveBeginPlay`
  (`KismetSystemLibrary.K2_SetTimerDelegate` (delegate `FireFlicker`) 0.05 true))

(event `FireFlicker`
  (`LightComponent.SetIntensity` (`self.PointLight`) (* (`KismetMathLibrary.FClamp` (`KismetMathLibrary.RandomFloat`) 0.4) 5000.0)))

(event `self.ReceiveTick`
  (params (DeltaSeconds :type "Float (single-precision)")))

(event `self.Sphere.OnComponentBeginOverlap`
  (params (OverlappedComponent :type "PrimitiveComponent Object Reference") (OtherActor :type "Actor Object Reference") (OtherComp :type "PrimitiveComponent Object Reference") (OtherBodyIndex :type Integer) (bFromSweep :type Boolean) (SweepResult :type "HitResult Structure (by ref)"))
  (`GameplayStatics.ApplyDamage` OtherActor 5.0))

(fn `UserConstructionScript`)