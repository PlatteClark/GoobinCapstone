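; BP_DayCycle is a day-night cycle that steps through four phases: Morning, Noon, Evening and Night.
; A looping timer, set by DayCycleLength in minutes per phase, calls ProgressTime, which also runs once at BeginPlay.
; Each step snaps SunLight to a fixed rotation and advances the phase, showing MoonLight at Night and hiding it at Morning.
; Each Morning also calls AgeUp on the player's BP_Character.
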(event `self.ReceiveBeginPlay`
  (`self.ProgressTime`)
  (`KismetSystemLibrary.K2_SetTimerDelegate` (delegate `ProgressTime`) (* (`self.DayCycleLength`) 60.0) true))

(event `ProgressTime`
  (switch `/Game/Goobin/Blueprints/Environment/E_DayCycle` (`self.EDayCycle`)
    (:`NewEnumerator0`
      (`SceneComponent.K2_SetWorldRotation` (`self.SunLight`) (struct :`Pitch` -20.0) false false)
      (set `self.EDayCycle` "NewEnumerator1")
      (`SceneComponent.SetVisibility` (`self.MoonLight`) false false)
      (`self.OnMorning`))
    (:`NewEnumerator1`
      (`SceneComponent.K2_SetWorldRotation` (`self.SunLight`) (struct :`Pitch` -80.0) false false)
      (set `self.EDayCycle` "NewEnumerator2"))
    (:`NewEnumerator2`
      (`SceneComponent.K2_SetWorldRotation` (`self.SunLight`) (struct :`Pitch` -20.0 :`Yaw` 180.0 :`Roll` 180.0) false false)
      (set `self.EDayCycle` "NewEnumerator3"))
    (:`NewEnumerator3`
      (`SceneComponent.K2_SetWorldRotation` (`self.SunLight`) (struct :`Pitch` 20.0) false false)
      (set `self.EDayCycle` "NewEnumerator0")
      (`SceneComponent.SetVisibility` (`self.MoonLight`) true false))))

(fn `OnMorning`
  (`/Game/Goobin/Blueprints/BP_Character.AgeUp` (cast `/Game/Goobin/Blueprints/BP_Character` (`GameplayStatics.GetPlayerCharacter` 0) :!pure true)))

(fn `UserConstructionScript`)