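; Base Blueprint for a harvestable node that drops items as it takes damage.
; AnyDamage scales damage by a DamageTable lookup keyed on the damage type's tool type, then passes it to the stats component.
; The component's OnDamaged event plays sound and Niagara effects and accumulates damage.
; Each full 100 accumulated spawns a random ItemSpawned class inside SpawnArea's bounds, carrying over the remainder.
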(event `self.ReceiveAnyDamage`
  (params (Damage :type "Float (single-precision)") (DamageType :type "DamageType Object Reference") (InstigatedBy :type "Controller Object Reference") (DamageCauser :type "Actor Object Reference"))
  (bind _tooltype (message `/Game/Goobin/Blueprints/BPI_Interactable.GetToolType` DamageType))
  (`/Game/Goobin/AC_Stats.AffectHealth` (`self.AC_Stats`) (* (`BlueprintMapLibrary.Map_Find` (`self.DamageTable`) _tooltype) Damage)))

(event `self.AC_Stats.OnDamaged`
  (params (Health :type "Float (double-precision)") (Damage :type "Float (double-precision)"))
  (bind _returnvalue (`self.K2_GetActorLocation`))
  (bind (_origin _boxextent) (`KismetSystemLibrary.GetComponentBounds` (`self.Spawn Area`)))
  (`GameplayStatics.PlaySoundAtLocation` (`self.SoundEffect`) _returnvalue (struct) 1.0 1.0 0.0 null null null null)
  (`NiagaraFunctionLibrary.SpawnSystemAtLocation` (`self.NiagaraEffect`) _returnvalue)
  (bind _output_get (set `self.AccumulatedDamage` (+ Damage (`self.AccumulatedDamage`))))
  (if (> _output_get 100.0)
    (for _ (range (+ (`KismetMathLibrary.FTrunc` (- (/ _output_get 100.0) 1.0)) 1))
      (`|SpawnActorFromClass` (`KismetArrayLibrary.Array_Random` (`self.ItemSpawned`)) (`KismetMathLibrary.MakeTransform` (`KismetMathLibrary.RandomPointInBoundingBox` _origin _boxextent)) "Undefined" "MultiplyWithRoot" null null))
    (set `self.AccumulatedDamage` (mod (`self.AccumulatedDamage`) 100.0))))

(fn `UserConstructionScript`)