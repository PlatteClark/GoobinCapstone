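; AC_ItemData is an actor component that turns its owner into a world item pickup identified by an item row and quantity.
; On begin play it makes the owning actor replicate.
; On Interact from a BP_Character, it adds the item to that character's AC inventory and destroys the owner if the add succeeds.
; Its LookAt function returns an empty string.
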(event `self.ReceiveBeginPlay`
  (`Actor.SetReplicates` (`self.GetOwner`) true))

(event `/Game/Goobin/Blueprints/BPI_Interactable.Interact`
  (params (Instigator :type "Actor Object Reference"))
  (bind (_itemid_datatable _itemid_rowname) (break `DataTableRowHandle` (`self.ItemID`)))
  (bind _asbp_character (cast `/Game/Goobin/Blueprints/BP_Character` Instigator))
  (bind _success (`/Game/Goobin/Inventory/AC_InventorySystem.AddToInventory` (`/Game/Goobin/Blueprints/BP_Character.AC_Inventory` _asbp_character) _itemid_rowname (`self.Quantity`)))
  (if _success
    (`Actor.K2_DestroyActor` (`self.GetOwner`))))

(fn `LookAt`
  (returns (Message :type Text))
  (return ""))