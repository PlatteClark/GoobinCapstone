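; BP_BoneSpear is a bone spear item that deals damage to actors it touches while active.
; When its capsule begins an overlap and IsActive is set, it applies fixed damage to the other actor with itself as causer and prints a debug hit message.
; An owner-tag check is left unconnected, so hits are not filtered by owner, and Tick is disabled.
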(event `self.Capsule.OnComponentBeginOverlap`
  (params (OverlappedComponent :type "PrimitiveComponent Object Reference") (OtherActor :type "Actor Object Reference") (OtherComp :type "PrimitiveComponent Object Reference") (OtherBodyIndex :type Integer) (bFromSweep :type Boolean) (SweepResult :type "HitResult Structure (by ref)"))
  (if (`self.IsActive`)
    (`GameplayStatics.ApplyDamage` OtherActor 50.0 null self)
    (`KismetSystemLibrary.PrintString` "target hit")))

(fn `UserConstructionScript`
  (`parent.UserConstructionScript`))