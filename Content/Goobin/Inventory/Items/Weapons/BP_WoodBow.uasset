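; BP_WoodBow is a usable bow item that fires an arrow when a character uses it.
; UseItem plays a montage on the character's skeletal mesh, then on blend out spawns a scaled BP_BoneArrow at the Arrow component and plays a release sound.
; The spawn keeps the Arrow component's roll but fixes pitch and adds a randomized negative yaw offset, giving shots horizontal spread.
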(event `/Game/Goobin/Blueprints/BPI_Interactable.UseItem`
  (params (Character :type "Actor Object Reference"))
  (bind _arrow (`self.Arrow`))
  (bind _returnvalue (`SceneComponent.K2_GetComponentLocation` _arrow))
  (bind (_returnvalue_roll _returnvalue_pitch _returnvalue_yaw) (`KismetMathLibrary.BreakRotator` (`SceneComponent.K2_GetComponentRotation` _arrow)))
  (`|PlayMontage` (`self.GetComponentByClass` Character "/Script/Engine.SkeletalMeshComponent") (`self.AnimToPlay`)
    (:`OnBlendOut`
      (`|SpawnActorFromClass` "/Game/Goobin/Inventory/Items/Weapons/BP_BoneArrow.BP_BoneArrow_C" (`KismetMathLibrary.MakeTransform` _returnvalue (`KismetMathLibrary.MakeRotator` _returnvalue_roll -85.0 (+ _returnvalue_yaw (`KismetMathLibrary.RandomFloatInRange` -35.0 -25.0))) (0.3 0.3 0.5)) "AlwaysSpawn" "MultiplyWithRoot" null null)
      (`GameplayStatics.PlaySoundAtLocation` "/Game/Goobin/Audio/Effects/Arrow_release.Arrow_release" _returnvalue (struct) 1.0 1.0 0.0 null null null null))))

(fn `UserConstructionScript`
  (`parent.UserConstructionScript`))