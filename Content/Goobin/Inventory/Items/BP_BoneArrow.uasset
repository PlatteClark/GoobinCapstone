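; BP_BoneArrow is a projectile arrow that damages what it hits and sticks into it.
; It has a 20-second lifespan and briefly disables collision on spawn before re-enabling it.
; Hits above a speed threshold apply damage.
; If the struck actor has a mesh component, the arrow attaches to it keeping world transform, stops projectile simulation and disables its collision.
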(event `self.ReceiveBeginPlay`
  (`self.SetLifeSpan` 20.0)
  (`self.SetActorEnableCollision` false)
  (`KismetSystemLibrary.Delay` 0.2)
  (`self.SetActorEnableCollision` true))

(event `self.ReceiveHit`
  (params (MyComp :type "PrimitiveComponent Object Reference") (Other :type "Actor Object Reference") (OtherComp :type "PrimitiveComponent Object Reference") (bSelfMoved :type Boolean) (HitLocation :type "Vector Structure") (HitNormal :type "Vector Structure") (NormalImpulse :type "Vector Structure") (Hit :type "HitResult Structure (by ref)"))
  (bind _returnvalue (`self.GetComponentByClass` Other "/Script/Engine.MeshComponent"))
  (if (> (`KismetMathLibrary.VSize` (`self.GetVelocity`)) 750.0)
    (`GameplayStatics.ApplyDamage` Other 25.0 null self)
    (`/Engine/EditorBlueprintResources/StandardMacros.IsValid` _returnvalue
      (:`Is Valid`
        (`self.K2_AttachToComponent` _returnvalue "None" "KeepWorld" "KeepWorld" "KeepWorld")
        (`ProjectileMovementComponent.StopSimulating` (`self.ProjectileMovement`) (`GameplayStatics.MakeHitResult` false true))
        (`self.SetActorEnableCollision` false)))))

(fn `UserConstructionScript`
  (`parent.UserConstructionScript`))