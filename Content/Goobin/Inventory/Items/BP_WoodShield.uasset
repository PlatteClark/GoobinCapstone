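; BP_WoodShield is a wooden shield inventory item that makes the character using it block damage.
; UseItem plays AnimToPlay on the character's skeletal mesh, and the montage's Notify Begin turns off Can Be Damaged and prints a debug string.
; The nodes that would restore Can Be Damaged and print "BlockEnded" are unconnected, so this Blueprint never ends the invulnerability.
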(event `/Game/Goobin/Blueprints/BPI_Interactable.UseItem`
  (params (Character :type "Actor Object Reference"))
  (`|PlayMontage` (`self.GetComponentByClass` Character "/Script/Engine.SkeletalMeshComponent") (`self.AnimToPlay`)
    (:`OnNotifyBegin`
      (set `Actor.bCanBeDamaged` false Character)
      (`KismetSystemLibrary.PrintString` "BlockStarted"))))

(fn `UserConstructionScript`
  (`parent.UserConstructionScript`))