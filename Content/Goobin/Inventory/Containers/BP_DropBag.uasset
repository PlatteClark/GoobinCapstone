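; BP_DropBag is a dropped inventory container that registers itself in level save data and disappears once emptied.
; On BeginPlay it adds its class and transform to the game mode's ActorsAdded save data and writes the level slot immediately.
; When its inventory component updates to zero quantity, it closes the HUD menu, records itself in ActorsRemoved without saving the slot, and destroys itself.
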(event `self.ReceiveBeginPlay`
  (bind (_returnvalue_location _returnvalue_rotation) (`KismetMathLibrary.BreakTransform` (`self.GetTransform`)))
  (bind _asbp_goobin_game_mode (cast `/Game/Goobin/BP_GoobinGameMode` (`GameplayStatics.GetGameMode`)))
  (bind _as_save_data_level (`/Game/Goobin/BP_GoobinGameMode.As Save Data Level` _asbp_goobin_game_mode))
  (`BlueprintMapLibrary.Map_Add` (`/Game/Goobin/SaveData_Level.ActorsAdded` _as_save_data_level) (`|ConvertAsset` (`GameplayStatics.GetObjectClass` self)) (`KismetMathLibrary.MakeTransform` _returnvalue_location _returnvalue_rotation))
  (`GameplayStatics.SaveGameToSlot` _as_save_data_level (`/Game/Goobin/BP_GoobinGameMode.LevelDataSlot` _asbp_goobin_game_mode)))

(event `self.AC_InventorySystem.OnInventoryUpdated`
  (if (<= (`/Game/Goobin/Inventory/AC_InventorySystem.GetQuantity` (`self.AC_InventorySystem`)) 0)
    (bind _asplayer_controller_goobin (cast `/Game/Goobin/Blueprints/PlayerController_Goobin` (`GameplayStatics.GetPlayerController` 0)))
    (`Widget.RemoveFromParent` (`/Game/Goobin/UI/W_HUD.Menu` (`/Game/Goobin/Blueprints/PlayerController_Goobin.HUD` _asplayer_controller_goobin)))
    (bind _asbp_goobin_game_mode (cast `/Game/Goobin/BP_GoobinGameMode` (`GameplayStatics.GetGameMode`)))
    (`KismetArrayLibrary.Array_AddUnique` (`/Game/Goobin/SaveData_Level.ActorsRemoved` (`/Game/Goobin/BP_GoobinGameMode.As Save Data Level` _asbp_goobin_game_mode)) (`|ConvertAsset` self))
    (`self.K2_DestroyActor`)))

(fn `UserConstructionScript`
  (`parent.UserConstructionScript`))