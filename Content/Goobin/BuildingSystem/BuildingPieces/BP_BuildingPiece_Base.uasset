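; Base actor for building pieces in the building system, handling the switch between placement preview and placed appearance.
; On BeginPlay it caches the static mesh's original materials and shows the invalid preview material.
; SetPreviewMaterial swaps every material slot to the good or bad preview material based on placement validity.
; PlaceObject restores the cached materials and ends previewing, but only when placement is valid.
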(event `self.ReceiveBeginPlay`
  (set `self.Materials` (`MeshComponent.GetMaterials` (`self.StaticMesh`)))
  (`self.SetPreviewMaterial` false))

(event `PlaceObject`
  (if (`self.IsValidPlacement`)
    (for (_array_element _array_index) (`self.Materials`)
      (`PrimitiveComponent.SetMaterial` (`self.StaticMesh`) _array_index _array_element))
    (set `self.IsPreviewing` false)))

(fn `SetPreviewMaterial`
  (params (IsValidPlacement :type Boolean))
  (set `self.PreviewMaterial` (select `bool` IsValidPlacement :`false` "/Game/Goobin/BuildingSystem/MI_BuildPreview_Bad.MI_BuildPreview_Bad" :`true` "/Game/Goobin/BuildingSystem/MI_BuildPreview_Good.MI_BuildPreview_Good" :!type "MaterialInterface Object Reference"))
  (for (_ _array_index) (`self.Materials`)
    (`PrimitiveComponent.SetMaterial` (`self.StaticMesh`) _array_index (`self.PreviewMaterial`))))

(fn `UserConstructionScript`)